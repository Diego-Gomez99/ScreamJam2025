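; Destructible barrel actor that breaks when damaged, drops loot and can optionally act as a readable clue.
; DoDamage fires once, spawning a destruction master field and each loot class at randomly scattered offsets, playing a break sound, then destroying the barrel after a delay.
; With ShowHint enabled, show/hide events toggle a prompt widget, and Interact toggles a clue text screen while disabling or restoring the player's movement.
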(event EventShowHUD
  (if (Variables|Default|GetShowHint)
    (Rendering|SetVisibility (Variables|Default|GetWidget) true false)))

(event EventHideHUD
  (if (Variables|Default|GetShowHint)
    (Rendering|SetVisibility (Variables|Default|GetWidget) false false)))

(event EventInteract
  (params (Player :type BP%20Third%20Person%20Character%20Object%20Reference))
  (Variables|Default|SetPlayer Player)
  (if (Variables|Default|GetShowHint)
    (if (Variables|Default|GetIsHUDSHOWING?)
      (Widget|RemovefromParent (Variables|Default|GetText_Widget))
      (Variables|Default|SetIsHUDSHOWING? false)
      (Pawn|Components|CharacterMovement|SetMovementMode (Variables|/Script/Engine.Character|GetCharacterMovement (Variables|Default|GetPlayer)) "MOVE_Walking" 0)
      (else
        (bind _returnvalue (UserInterface|CreateWidget "/Game/Widgets_HUD/TEXT_Widget.TEXT_Widget_C"))
        (bind _output_get (Variables|Default|SetText_Widget _returnvalue))
        (UserInterface|Viewport|AddtoViewport _output_get 0)
        (Variables|/Script/UMG.TextBlock|SetText (Variables|/Game/Widgets_HUD/TEXT_Widget.TEXT_Widget_C|GetClue_Text_Widget (Variables|Default|GetText_Widget)) (Variables|Default|GetClue_Text))
        (Pawn|Components|CharacterMovement|SetMovementMode (Variables|/Script/Engine.Character|GetCharacterMovement (Variables|Default|GetPlayer)) "MOVE_None" 0)
        (Variables|Default|SetIsHUDSHOWING? true)))))

(event EventDoDamage
  (params (HitLocation :type Vector :default "0, 0, 0"))
  (bind _returnvalue (Math|Random|RandomFloatinRange -1e+02 8e+01))
  (bind _returnvalue_2 (Transformation|GetActorLocation))
  (if (not (Variables|Default|GetDestroyed))
    (Development|PrintString "Destroyed" true true "(R=1.000000,G=0.000000,B=0.157705,A=1.000000)")
    (Variables|Default|SetDestroyed true)
    (Game|SpawnActorfromClass "/Game/DestructionMasterField_BP.DestructionMasterField_BP_C" (Math|Conversions|ToTransform(Vector) (Transformation|GetActorLocation)) "Undefined" "MultiplyWithRoot" 0 0)
    (for _array_element (Variables|Default|GetArrayLoot)
      (Game|SpawnActorfromClass _array_element (Math|Transform|MakeTransform (Math|Vector|MakeVector (+ (.x _returnvalue_2) _returnvalue) (+ (.y _returnvalue_2) _returnvalue) (.z _returnvalue_2)) "0, 0, 0" "1.000000,1.000000,1.000000") "Undefined" "MultiplyWithRoot" 0 0))
    (Audio|Components|Audio|Play (Variables|Default|GetWood+Box+Break) 0.0)
    (Utilities|FlowControl|Delay 3.0)
    (Actor|DestroyActor)))

(fn ConstructionScript)