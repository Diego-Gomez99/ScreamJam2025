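; BP_MusicZone is a trigger zone that plays a music track as 2D audio while the player is inside it.
; An overlap by an actor tagged Player spawns the Music sound and fades it in, and leaving fades out the stored sound.
; The StartSong flag also starts the track on BeginPlay.
; Each start spawns a fresh sound and overwrites the stored reference without stopping the previous one.
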(event OnComponentBeginOverlap(Trigger)
  (params (OverlappedComponent :type Primitive%20Component%20Object%20Reference) (OtherActor :type Actor%20Object%20Reference) (OtherComp :type Primitive%20Component%20Object%20Reference) (OtherBodyIndex :type Integer) (bFromSweep :type Boolean) (SweepResult :type Hit%20Result%20Structure%20%28by%20ref%29))
  (if (Actor|ActorHasTag OtherActor "Player")
    (bind _music (Variables|Default|GetMusic)
      (:then
        (bind _returnvalue (Audio|SpawnSound2D _music 0.3 1.0 0.0 0))
        (bind _output_get (Variables|Default|SetNewSound _returnvalue))
        (Audio|Components|Audio|FadeIn _output_get 0.5 0.5 0.0 "Linear" :!class /Script/Engine.AudioComponent))
      (:else))))

(event OnComponentEndOverlap(Trigger)
  (params (OverlappedComponent :type Primitive%20Component%20Object%20Reference) (OtherActor :type Actor%20Object%20Reference) (OtherComp :type Primitive%20Component%20Object%20Reference) (OtherBodyIndex :type Integer))
  (if (Actor|ActorHasTag OtherActor "Player")
    (bind _newsound (Variables|Default|GetNewSound)
      (:then
        (Audio|Components|Audio|FadeOut _newsound 0.5 0.0 "Linear" :!class /Script/Engine.AudioComponent))
      (:else))))

(event EventBeginPlay
  (if (Variables|Default|GetStartSong?)
    (bind _music (Variables|Default|GetMusic)
      (:then
        (bind _returnvalue (Audio|SpawnSound2D _music 0.3 1.0 0.0 0))
        (bind _output_get (Variables|Default|SetNewSound _returnvalue))
        (Audio|Components|Audio|FadeIn _output_get 0.5 0.5 0.0 "Linear" :!class /Script/Engine.AudioComponent))
      (:else))))

(fn ConstructionScript)