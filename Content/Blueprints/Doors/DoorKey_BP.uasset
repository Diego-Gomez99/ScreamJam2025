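; DoorKey_BP is a key-locked door that teleports the player to its other side once unlocked.
; Picking up the key unlocks it, and BeginPlay restores that state from the save game in Slot_01.
; Interacting when open teleports the player to the farther of two arrow components, masked by a camera fade and door sounds.
; When locked, interacting toggles a clue text widget and disables player movement while it shows.
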(event EventPickUpKey
  (bind _output_get (Variables|Default|SetHasKey true))
  (Variables|Default|SetIsOpen _output_get))

(event EventBeginPlay
  (CallFunction|LoadInfo))

(event EventInteract
  (params (Player :type BP%20Third%20Person%20Character%20Object%20Reference))
  (Variables|Default|SetPlayer Player)
  (if (Variables|Default|GetIsOpen)
    ;[1 1 1 0.157] Open / Close Door
    (bind _arrowtoteleport (CallFunction|GetArrowtoTeleport (Variables|Default|GetPlayer)))
    (CameraFades|StartCameraFade :self (Variables|/Script/Engine.PlayerController|GetPlayerCameraManager (Game|GetPlayerController 0)) :ToAlpha 1.0 :Duration 0.5)
    (Audio|PlaySound2D "/Game/Sounds/Door/Open_Door.Open_Door" 1.0 1.0 0.0 0 0)
    (Utilities|FlowControl|Delay 0.5)
    (Transformation|SetActorLocation (Variables|Default|GetPlayer) _arrowtoteleport false true)
    (Audio|PlaySound2D "/Game/Sounds/Door/Door_Closed.Door_Closed" 1.0 1.0 0.0 0 0)
    (CameraFades|StartCameraFade :self (Variables|/Script/Engine.PlayerController|GetPlayerCameraManager (Game|GetPlayerController 0)) :FromAlpha 1.0 :Duration 0.5)
    (elif (Variables|Default|GetIsShowingHUD)
      (Widget|RemovefromParent (Variables|Default|GetTEXT%20Widget))
      (Variables|Default|SetIsShowingHUD false)
      (Pawn|Components|CharacterMovement|SetMovementMode (Variables|/Script/Engine.Character|GetCharacterMovement (Variables|Default|GetPlayer)) "MOVE_Walking" 0)
      (else
        (bind _returnvalue (UserInterface|CreateWidget "/Game/Widgets_HUD/TEXT_Widget.TEXT_Widget_C"))
        (bind _output_get (Variables|Default|SetTEXT%20Widget _returnvalue))
        (UserInterface|Viewport|AddtoViewport _output_get 0)
        (Variables|/Script/UMG.TextBlock|SetText (Variables|/Game/Widgets_HUD/TEXT_Widget.TEXT_Widget_C|GetClue_Text_Widget (Variables|Default|GetTEXT%20Widget)) (Variables|Default|GetClue%20Text))
        (Variables|Default|SetIsShowingHUD true)
        (Pawn|Components|CharacterMovement|SetMovementMode (Variables|/Script/Engine.Character|GetCharacterMovement (Variables|Default|GetPlayer)) "MOVE_None" 0)))))

(fn ConstructionScript)

(fn GetArrowtoTeleport
  (params (Player :type Actor%20Object%20Reference))
  (bind _output_get (Variables|Default|SetPlayerLocation (Transformation|GetActorLocation Player)))
  (Variables|Default|SetArrow1_Distance (Math|Vector|Distance(Vector) _output_get (Transformation|GetWorldLocation (Variables|Default|GetArrow1))))
  (Variables|Default|SetArrow2_Distance (Math|Vector|Distance(Vector) (Variables|Default|GetPlayerLocation) (Transformation|GetWorldLocation (Variables|Default|GetArrow))))
  (if (< (Variables|Default|GetArrow1_Distance) (Variables|Default|GetArrow2_Distance))
    (return (Transformation|GetWorldLocation (Variables|Default|GetArrow)))
    (else
      (return (Transformation|GetWorldLocation (Variables|Default|GetArrow1))))))

(fn LoadInfo
  (bind _returnvalue (SaveGame|DoesSaveGameExist "Slot_01"))
  (if _returnvalue
    (bind _returnvalue_2 (SaveGame|LoadGamefromSlot "Slot_01"))
    (bind _assave_game_bp (Utilities|Casting|CastToSaveGame_BP _returnvalue_2))
    (Variables|Default|SetIsOpen (Variables|/Game/Blueprints/SaveGame_BP.SaveGame_BP_C|GetIsDoorOpen? _assave_game_bp))
    (else
      (Development|PrintString "Not Found" true true "(R=1.000000,G=0.017520,B=0.000000,A=1.000000)"))))