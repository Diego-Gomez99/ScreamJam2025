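; Bandages pickup actor that heals the interacting player.
; Interact passes HealAmount to the player's FillHeal and destroys the actor only if that call returns true.
; ShowHUD and HideHUD are empty, leaving the Interaction_Widget prompt text and visibility logic disconnected in the graph.
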(event EventShowHUD)

(event EventHideHUD)

(event EventInteract
  (params (Player :type BP%20Third%20Person%20Character%20Object%20Reference))
  (bind _destroy_ (Default|FillHeal Player (Variables|Default|GetHealAmount)))
  (if _destroy_
    (Actor|DestroyActor)))

(fn ConstructionScript)