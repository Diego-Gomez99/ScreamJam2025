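; Interactable control panel that opens a linked door once the correct code is entered on a keypad widget.
; Interact toggles via FlipFlop between showing the code pad with cursor and frozen player movement, and closing it to restore control.
; The widget receives the password and a panel reference.
; CorrectPassword closes it, restores control, sets the door's IsOpen and marks the panel unlocked, blocking further interaction.
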(event EventInteract
  (params (Player :type BP%20Third%20Person%20Character%20Object%20Reference))
  (bind _returnvalue (Game|GetPlayerController 0))
  (if (not (Variables|Default|GetUnlocked?))
    (Variables|Default|SetPlayer Player)
    (Utilities|FlowControl|FlipFlop
      (:A
        (bind _returnvalue_2 (UserInterface|CreateWidget "/Game/Widgets_HUD/CombinationDoor_widget.CombinationDoor_widget_C"))
        (Variables|Default|SetCodePadWidget _returnvalue_2)
        (UserInterface|Viewport|AddtoViewport _returnvalue_2 0)
        (Input|SetInputModeGameandUI _returnvalue _returnvalue_2 "DoNotLock" true false)
        (Variables|/Script/Engine.PlayerController|SetbShowMouseCursor _returnvalue true)
        (Pawn|Components|CharacterMovement|SetMovementMode (Variables|/Script/Engine.Character|GetCharacterMovement (Variables|Default|GetPlayer)) "MOVE_None" 0)
        (Variables|/Game/Widgets_HUD/CombinationDoor_widget.CombinationDoor_widget_C|SetPassword (Variables|Default|GetCodePadWidget) (Variables|Default|GetPassword))
        (Variables|/Game/Widgets_HUD/CombinationDoor_widget.CombinationDoor_widget_C|SetControlPanel_BP (Variables|Default|GetCodePadWidget) self))
      (:B
        (Widget|RemovefromParent _returnvalue_2)
        (Input|SetInputModeGameOnly _returnvalue false)
        (Variables|/Script/Engine.PlayerController|SetbShowMouseCursor _returnvalue false)
        (Pawn|Components|CharacterMovement|SetMovementMode (Variables|/Script/Engine.Character|GetCharacterMovement (Variables|Default|GetPlayer)) "MOVE_Walking" 0)))))

(fn ConstructionScript)

(fn CorrectPassword
  (bind _returnvalue (Game|GetPlayerController 0))
  (Widget|RemovefromParent (Variables|Default|GetCodePadWidget))
  (Input|SetInputModeGameOnly _returnvalue false)
  (Variables|/Script/Engine.PlayerController|SetbShowMouseCursor _returnvalue false)
  (Pawn|Components|CharacterMovement|SetMovementMode (Variables|/Script/Engine.Character|GetCharacterMovement (Variables|Default|GetPlayer)) "MOVE_Walking" 0)
  (bind _output_get (Variables|/Game/Blueprints/Doors/Control_Panel_Door_BP.Control_Panel_Door_BP_C|SetIsOpen (Variables|Default|GetControl_Panel_Door) true))
  (Variables|Default|SetUnlocked? _output_get))