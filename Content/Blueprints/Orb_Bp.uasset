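; Orb_Bp is an interactable orb actor that triggers a number display on a tank and is consumed on use.
; Interact clears the player's InteractActor reference, calls ShowNumber on the referenced TankBP and destroys the orb.
; ShowHUD writes TextMessage into the Interaction_Widget held by its widget component and makes it visible, while HideHUD hides it.
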(event EventInteract
  (params (Player :type BP%20Third%20Person%20Character%20Object%20Reference))
  (Variables|/Game/ThirdPerson/Blueprints/BP_ThirdPersonCharacter.BP_ThirdPersonCharacter_C|SetInteract_Actor Player 0)
  (Default|ShowNumber (Variables|Default|GetTank_BP))
  (Actor|DestroyActor))

(event EventShowHUD
  (bind _asinteraction_widget (Utilities|Casting|CastToInteraction_Widget (UserInterface|GetWidget (Variables|Default|GetWidget))))
  (Variables|/Script/UMG.TextBlock|SetText (Variables|/Game/Widgets_HUD/Interaction_Widget.Interaction_Widget_C|GetText_Interact_Name _asinteraction_widget) (Variables|Default|GetText%20Message))
  (Rendering|SetVisibility (Variables|Default|GetWidget) true false))

(event EventHideHUD
  (Rendering|SetVisibility (Variables|Default|GetWidget) false false))

(fn ConstructionScript)