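; SaveSystem is an interactable Blueprint that toggles a save menu for the player who uses it.
; Its Interact event stores the player and runs a FlipFlop that alternately creates a new Save_Widget or removes it from the viewport.
; Opening shows the cursor, sets Game and UI input and disables character movement, while closing restores game-only input and walking.
; The Blueprint itself contains no save or load logic.
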(event EventInteract
  (params (Player :type BP%20Third%20Person%20Character%20Object%20Reference))
  (bind _returnvalue (Game|GetPlayerController 0))
  (Variables|Default|SetPlayer Player)
  (Utilities|FlowControl|FlipFlop
    (:A
      (bind _returnvalue_2 (UserInterface|CreateWidget "/Game/Widgets_HUD/Save_Widget.Save_Widget_C"))
      (bind _output_get (Variables|Default|SetSaveWidget _returnvalue_2))
      (UserInterface|Viewport|AddtoViewport _output_get 0)
      (Input|SetInputModeGameandUI _returnvalue (Variables|Default|GetSaveWidget) "DoNotLock" true false)
      (Variables|/Script/Engine.PlayerController|SetbShowMouseCursor _returnvalue true)
      (Pawn|Components|CharacterMovement|SetMovementMode (Variables|/Script/Engine.Character|GetCharacterMovement (Variables|Default|GetPlayer)) "MOVE_None" 0))
    (:B
      (Widget|RemovefromParent _output_get)
      (Input|SetInputModeGameOnly _returnvalue false)
      (Variables|/Script/Engine.PlayerController|SetbShowMouseCursor _returnvalue false)
      (Pawn|Components|CharacterMovement|SetMovementMode (Variables|/Script/Engine.Character|GetCharacterMovement (Variables|Default|GetPlayer)) "MOVE_Walking" 0))))

(fn ConstructionScript)